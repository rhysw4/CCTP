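; Base dialogue component for NPCs that opens and closes the dialogue widget, disabling player movement while it is shown.
; Child classes script conversations by overriding the empty Dialogue function with AddDialogue calls.
; Each option choice is stored by step index and Dialogue replays from the start, with AddDialogue returning saved choices or displaying unanswered lines.
; Helpers clear or rewind progress and switch the dialogue tree index.
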(fn OpenDialogue
  (Utilities|FlowControl|Sequence
    (:then_0
      ;[0.15 0.15 0.15 0.5] create dialogue widget
      (bind _returnvalue (UserInterface|CreateWidget "/Game/DialogueSystem2/NPC_Base2/UI/WB_Dialogue2.WB_Dialogue2_C" 0 self))
      (bind _output_get (Variables|Default|SetDialogueWidget _returnvalue))
      (UserInterface|Viewport|AddtoViewport _output_get 0)
      (CallFunction|ProgressDialogue))
    (:then_1
      ;[0.15 0.15 0.15 0.5] disable character movement
      (bind _ascharacter (Utilities|Casting|CastToCharacter (Game|GetPlayerCharacter 0)))
      (Pawn|Components|CharacterMovement|DisableMovement (Variables|/Script/Engine.Character|GetCharacterMovement _ascharacter))
      (Variables|/Script/Engine.PlayerController|SetbShowMouseCursor (Game|GetPlayerController 0) true))))

(fn CloseDialogue
  (Utilities|FlowControl|Sequence
    (:then_0
      ;[0.15 0.15 0.15 0.5] remove dialogue widget
      (Widget|RemovefromParent (Variables|Default|GetDialogueWidget)))
    (:then_1
      ;[0.15 0.15 0.15 0.5] enable character movement
      (bind _ascharacter (Utilities|Casting|CastToCharacter (Game|GetPlayerCharacter 0)))
      (Pawn|Components|CharacterMovement|SetMovementMode (Variables|/Script/Engine.Character|GetCharacterMovement _ascharacter) "MOVE_Walking" 0))))

(fn ProgressDialogue
  (Variables|Default|SetDialogueIndex -1)
  (CallFunction|Dialogue))

(fn Dialogue)

(fn AddDialogue
  (params (SpeakerName :type Text) (SpeakerDialogue :type Text) (OptionText :type Array%20of%20Texts))
  (bind _dialogueprogress (Variables|Default|GetDialogueProgress))
  (bind _dialogueindex (Variables|Default|GetDialogueIndex))
  (bind (_value _returnvalue) (Utilities|Map|Find _dialogueprogress _dialogueindex))
  ;[0.15 0.15 0.15 0.5] add dialogue
  (Math|Integer|IncrementInt (Variables|Default|GetDialogueIndex)
    (:%20%20
      (if _returnvalue
        (return "NewEnumerator0" _value)
        (else
          ;[0.15 0.15 0.15 0.5] update added dialogue
          (Default|UpdateDialogueText (Variables|Default|GetDialogueWidget) (Variables|Default|GetDialogueIndex) SpeakerName SpeakerDialogue OptionText)
          (return "NewEnumerator1" 0))))))

(fn UpdateSelectedOption
  (params (ProgressIndex :type Integer%20%28by%20ref%29) (OptionIndex :type Integer%20%28by%20ref%29))
  ;[0.15 0.15 0.15 0.5] update dialogue
  (Utilities|Map|Add (Variables|Default|GetDialogueProgress) ProgressIndex OptionIndex)
  (CallFunction|ProgressDialogue))

(fn ClearDialogueProgress
  ;[0.15 0.15 0.15 0.5] clear dialogue progress
  (Utilities|Map|Clear (Variables|Default|GetDialogueProgress)))

(fn RemoveDialoguePogress
  (params (ProgressSteps :type Integer))
  ;[0.15 0.15 0.15 0.5] remove dialogue progress
  (for _index (range 0 ProgressSteps)
    (Utilities|Map|Remove (Variables|Default|GetDialogueProgress) (- (Variables|Default|GetDialogueIndex) _index))))

(fn SetDialogueTreeIndex
  (params (DialogueTreeIndex :type Integer))
  ;[0.15 0.15 0.15 0.5] set tree index
  (Variables|Default|SetDialogueTreeIndex DialogueTreeIndex)
  (CallFunction|ClearDialogueProgress))