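; Player interaction component that tracks nearby interactable actors and lets the owning character interact with one of them.
; Capsule begin and end overlaps add or remove actors implementing BPI_Interact, treating the most recently added as active.
; A screen-space widget component, created at BeginPlay, shows a fresh WB_Interact at the active actor's location, refreshed on each overlap change.
; The IA_Interact input sends that actor an interact message with the owner.
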(event Custom|CapsuleOverlapBeginEvent
  (params (OverlappedComponent :type Primitive%20Component%20Object%20Reference) (OtherActor :type Actor%20Object%20Reference) (OtherComp :type Primitive%20Component%20Object%20Reference) (OtherBodyIndex :type Integer) (bFromSweep :type Boolean) (SweepResult :type Hit%20Result%20Structure%20%28by%20ref%29))
  (if (Utilities|DoesObjectImplementInterface OtherActor "/Game/InteractionSystem/BPI_Interact.BPI_Interact_C")
    (Utilities|Array|AddUnique (Variables|Default|GetInteractablesInRange) OtherActor)
    (CallFunction|RenderWidget)))

(event Custom|CapsuleOverlapEndEvent
  (params (OverlappedComponent :type Primitive%20Component%20Object%20Reference) (OtherActor :type Actor%20Object%20Reference) (OtherComp :type Primitive%20Component%20Object%20Reference) (OtherBodyIndex :type Integer))
  (if (Utilities|DoesObjectImplementInterface OtherActor "/Game/InteractionSystem/BPI_Interact.BPI_Interact_C")
    (Utilities|Array|RemoveItem (Variables|Default|GetInteractablesInRange) OtherActor)
    (CallFunction|RenderWidget)))

(event Input|EnhancedActionEvents|EnhancedInputActionIA_Interact
  (params (ActionValue :type Boolean) (ElapsedSeconds :type Float%20%28double-precision%29) (TriggeredSeconds :type Float%20%28double-precision%29) (InputAction :type Input%20Action%20Object%20Reference :default "/Game/Input/Actions/IA_Interact.IA_Interact"))
  (:Started
    (Class|BPIInteract|Interact(Message) (CallFunction|GetActiveInteractable) (Components|GetOwner))))

(event EventBeginPlay
  (bind _ascharacter (Utilities|Casting|CastToCharacter (Components|GetOwner)))
  (Collision|BindEventtoOnComponentBeginOverlap (Variables|/Script/Engine.Character|GetCapsuleComponent _ascharacter) (EventDispatchers|CreateEvent :!event Custom|CapsuleOverlapBeginEvent))
  (Collision|BindEventtoOnComponentEndOverlap (Variables|/Script/Engine.Character|GetCapsuleComponent _ascharacter) (EventDispatchers|CreateEvent :!event Custom|CapsuleOverlapEndEvent))
  (bind _returnvalue (Game|AddComponentbyClass (Components|GetOwner) "/Script/UMG.WidgetComponent" true))
  (Class|WidgetComponent|SetWidgetSpace _returnvalue "Screen")
  (Class|WidgetComponent|SetDrawSize _returnvalue "(X=250.000000,Y=50.000000)")
  (Variables|Default|SetInteractionWidgetComponent _returnvalue))

(fn RenderWidget
  (bind _activeinteractable (CallFunction|GetActiveInteractable))
  (bind _interactionwidgetcomponent (Variables|Default|GetInteractionWidgetComponent))
  (bind _returnvalue (Transformation|GetActorLocation _activeinteractable))
  (if (Utilities|Array|IsNotEmpty (Variables|Default|GetInteractablesInRange))
    (bind _returnvalue_2 (UserInterface|CreateWidget "/Game/InteractionSystem/WB_Interact.WB_Interact_C"))
    (UserInterface|SetWidget _interactionwidgetcomponent _returnvalue_2)
    (Transformation|SetWorldLocation _interactionwidgetcomponent (Math|Vector|MakeVector (.x _returnvalue) (.y _returnvalue) (.z _returnvalue)) false false)
    (else
      (UserInterface|SetWidget (Variables|Default|GetInteractionWidgetComponent) 0))))

(fn GetActiveInteractable
  (bind _interactablesinrange (Variables|Default|GetInteractablesInRange))
  (return (Utilities|Array|Get(acopy) _interactablesinrange (Utilities|Array|LastIndex _interactablesinrange))))