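; BP_Door is an interactable door in the interaction system that swings open and closed.
; Its Interact event checks the IsOpen flag and calls DoorOpen or DoorClose.
; A single timeline drives the door's relative yaw, playing forward to open and in reverse to close.
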(event Custom|DoorOpen
  ;[0.15 0.15 0.15 0.5] Open Close Door
  (Variables|Default|SetisOpen true)
  (bind _zrotation (Timeline|DoorOpenTimeline Play)
    (:Update
      (Transformation|SetRelativeRotation (Variables|Default|GetDoor) (Math|Rotator|MakeRotator 0.0 0.0 _zrotation) false false))))

(event Custom|DoorClose
  ;[0.15 0.15 0.15 0.5] Open Close Door
  (Variables|Default|SetisOpen false)
  (bind _zrotation (Timeline|DoorOpenTimeline Reverse)
    (:Update
      (Transformation|SetRelativeRotation (Variables|Default|GetDoor) (Math|Rotator|MakeRotator 0.0 0.0 _zrotation) false false))))

(event EventInteract
  (params (Interactor :type Actor%20Object%20Reference))
  ;[0.15 0.15 0.15 0.5] Check door open close
  (if (Variables|Default|GetisOpen)
    (CallFunction|DoorClose)
    (else
      (CallFunction|DoorOpen))))

(fn ConstructionScript)