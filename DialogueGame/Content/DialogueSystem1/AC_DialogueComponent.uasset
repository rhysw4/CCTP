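; Dialogue component that steps through a conversation one line per Interact call, shown in a WB_Dialogue widget.
; The first call creates the widget with the speaker name and row text; later calls update the existing widget.
; Each data table row supplies the next row name, table and end flag, so conversations chain across tables.
; Once the end flag is set, the following Interact removes the widget and clears its reference.
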(event EventInteract
  (params (PlayerReference :type BP%20Third%20Person%20Character%20Object%20Reference))
  (if (Variables|Default|GetEndDialogue)
    (Widget|RemovefromParent (Variables|Default|GetDialogue%20Widget))
    (Variables|Default|SetEndDialogue false)
    (Variables|Default|SetDialogue%20Widget 0)
    (else
      (Development|PrintString "STARTING")
      (Utilities|IsValid (Variables|Default|GetDialogue%20Widget)
        (:Is%20Valid
          ;[0.15 0.15 0.15 0.5] Error Here
          (bind _returnvalue (Utilities|GetDataTableRow (Variables|Default|GetData%20Table) (Variables|Default|GetRow%20Name))
            (:then
              (Development|PrintString "GOING TO UPDATE")
              ;;[0.15 0.15 0.15 0.5] Error
              (Default|UpdateDialogue (Variables|Default|GetDialogue%20Widget) (.Dialogue (Utilities|Struct|BreakS_Dialogue _returnvalue)))
              (Development|PrintString "IS UPDATING DIALOGUE")
              (Variables|Default|SetRow%20Name (.Row (Utilities|Struct|BreakS_Dialogue _returnvalue)))
              (Variables|Default|SetData%20Table (.DataTable (Utilities|Struct|BreakS_Dialogue _returnvalue)))
              (Variables|Default|SetEndDialogue (.EndDialogue (Utilities|Struct|BreakS_Dialogue _returnvalue))))
            (:RowNotFound
              (Development|PrintString "BWOKEN"))))
        (:Is%20Not%20Valid
          (bind _returnvalue_2 (Utilities|GetDataTableRow (Variables|Default|GetData%20Table) (Variables|Default|GetRow%20Name))
            (:then
              (Development|PrintString "IT WORKS")
              (bind _returnvalue_3 (UserInterface|CreateWidget "/Game/DialogueSystem1/WB_Dialogue.WB_Dialogue_C" 0 (Utilities|Text|ToText(Name) (Variables|Default|GetName)) (.Dialogue (Utilities|Struct|BreakS_Dialogue _returnvalue_2))))
              (bind _output_get (Variables|Default|SetDialogue%20Widget _returnvalue_3))
              (UserInterface|Viewport|AddtoViewport _output_get 0)
              (Variables|Default|SetRow%20Name (.Row (Utilities|Struct|BreakS_Dialogue _returnvalue_2)))
              (Variables|Default|SetData%20Table (.DataTable (Utilities|Struct|BreakS_Dialogue _returnvalue_2)))
              (Variables|Default|SetEndDialogue (.EndDialogue (Utilities|Struct|BreakS_Dialogue _returnvalue_2))))
            (:RowNotFound
              (Development|PrintString "IT BROKE"))))))))