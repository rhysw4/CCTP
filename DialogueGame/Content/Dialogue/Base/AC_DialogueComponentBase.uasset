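; Base dialogue component that runs branching conversations through a WB_Dialogue widget, with an empty Dialogue function as the script hook.
; Each progress step resets the index and replays Dialogue from the top.
; AddDialogue returns stored choices for answered lines and sends unanswered ones to the widget.
; UpdateSelectedOption records choices and replays; helpers remove or clear progress, including when the tree index is set.
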(fn OpenConversation
  ;[1 1 1] Open Conversation
  (bind _returnvalue (UserInterface|CreateWidget "/Game/UI/DialogueUI/WB_Dialogue.WB_Dialogue_C" 0 self))
  (bind _output_get (Variables|Default|SetDialogueWidget _returnvalue))
  (UserInterface|Viewport|AddtoViewport _output_get 0)
  (CallFunction|ProgressDialogue))

(fn CloseConversation
  ;[1 1 1] Close Conversation
  (Widget|RemovefromParent (Variables|Default|GetDialogueWidget)))

(fn ProgressDialogue
  (Variables|Default|SetDialogueIndex -1)
  (CallFunction|Dialogue))

(fn Dialogue)

(fn AddDialogue
  (params (Speaker :type Text) (Dialogue :type Text) (OptionsText :type Array%20of%20Texts))
  (bind _dialogueprogress (Variables|Default|GetDialogueProgress))
  (bind _dialogueindex (Variables|Default|GetDialogueIndex))
  (bind (_value _returnvalue) (Utilities|Map|Find _dialogueprogress _dialogueindex))
  ;[1 1 1] Add Dialogue
  (Math|Integer|IncrementInt (Variables|Default|GetDialogueIndex)
    (:%20%20
      (if _returnvalue
        (return "NewEnumerator0" _value)
        (else
          (Default|UpdateDialogueText (Variables|Default|GetDialogueWidget) (Variables|Default|GetDialogueIndex) Speaker Dialogue OptionsText)
          (return "NewEnumerator4" 0))))))

(fn UpdateSelectedOption
  (params (ProgressIndex :type Integer%20%28by%20ref%29) (OptionsIndex :type Integer%20%28by%20ref%29))
  ;[1 1 1] Update Options
  (Utilities|Map|Add (Variables|Default|GetDialogueProgress) ProgressIndex OptionsIndex)
  (CallFunction|ProgressDialogue))

(fn ClearDialogueProgress
  ;[1 1 1] Clear Dialogue
  (Utilities|Map|Clear (Variables|Default|GetDialogueProgress)))

(fn RemoveDialogueProgress
  (params (ProgressSteps :type Integer))
  ;[1 1 1] Remove Dialogue
  (for _index (range 0 ProgressSteps)
    (Utilities|Map|Remove (Variables|Default|GetDialogueProgress) (- (Variables|Default|GetDialogueIndex) _index))))

(fn SetDialogueTreeIndex
  (params (DialogueTreeIndex :type Integer))
  ;[1 1 1] Set Tree Index
  (Variables|Default|SetDialogueTreeIndex DialogueTreeIndex)
  (CallFunction|ClearDialogueProgress))