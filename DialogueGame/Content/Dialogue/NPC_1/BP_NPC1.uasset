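; NPC Blueprint that runs a data-table-driven, branching conversation when a character interacts with it.
; Interact disables player movement, then creates the dialogue widget or advances it, and closes it and restores control once a row flags the end.
; Each row links to the next row and table.
; Branching rows spawn option widgets on the first line and after OptionSelected, but not when Interact advances an open dialogue.
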(event Custom|OptionSelected
  (params (RowName :type Name) (DataTable :type Data%20Table%20Object%20Reference))
  (bind _dialoguewidget (Variables|Default|GetDialogueWidget))
  ;[0.15 0.15 0.15 0.5] Select option and update dialogue and the options
  (bind _returnvalue (Utilities|GetDataTableRow DataTable RowName)
    (:then
      (Widget|Panel|ClearChildren (Variables|/Game/Dialogue/WB_Dialogue.WB_Dialogue_C|GetOptionsScrollBox _dialoguewidget))
      (Default|UpdateDialogue _dialoguewidget (.Dialogue (Utilities|Struct|BreakS_Dialogue _returnvalue)))
      (Variables|Default|SetRow%20Name (.Row (Utilities|Struct|BreakS_Dialogue _returnvalue)))
      (Variables|Default|SetData%20Table (.DataTable (Utilities|Struct|BreakS_Dialogue _returnvalue)))
      (Variables|Default|SetEndDialogue (.EndDialogue (Utilities|Struct|BreakS_Dialogue _returnvalue)))
      (if (.OpenendedDialogue (Utilities|Struct|BreakS_Dialogue _returnvalue))
        (for _array_element (.OpenendedDialogueOptions (Utilities|Struct|BreakS_Dialogue _returnvalue))
          (bind _returnvalue_2 (UserInterface|CreateWidget "/Game/Dialogue/WB_Options.WB_Options_C" 0 (Utilities|Text|ToText(Name) (.OptionName (Utilities|Struct|BreakS_OptionsDialogue _array_element))) self (.Row (Utilities|Struct|BreakS_OptionsDialogue _array_element)) (.DataTable (Utilities|Struct|BreakS_OptionsDialogue _array_element))))
          (Widget|Panel|AddChild (Variables|/Game/Dialogue/WB_Dialogue.WB_Dialogue_C|GetOptionsScrollBox (Variables|Default|GetDialogueWidget)) _returnvalue_2))))))

(event EventInteract
  (params (Interactor :type Actor%20Object%20Reference))
  (bind _returnvalue (Game|GetPlayerController 0))
  (bind _returnvalue_2 (Game|GetPlayerController 0))
  ;[0.15 0.15 0.15 0.5] Interacting with Character
  (Utilities|Casting|CastToCharacter Interactor)
  ;[0.15 0.15 0.15 0.5] Disable movement
  (Pawn|Components|CharacterMovement|DisableMovement (Variables|/Script/Engine.Character|GetCharacterMovement (Game|GetPlayerCharacter 0)))
  ;[0.15 0.15 0.15 0.5] Is Dialogue Ending?
  (if (Variables|Default|GetEndDialogue)
    ;[0.15 0.15 0.15 0.5] Dialogue Ended
    (Widget|RemovefromParent (Variables|Default|GetDialogueWidget))
    (Variables|Default|SetEndDialogue false)
    (Variables|Default|SetDialogueWidget 0)
    ;[0.15 0.15 0.15 0.5] Enable movement, hide cursor, input mode
    (bind _ascharacter (Utilities|Casting|CastToCharacter Interactor))
    (Pawn|Components|CharacterMovement|SetMovementMode (Variables|/Script/Engine.Character|GetCharacterMovement _ascharacter) "MOVE_Walking" 0)
    (Variables|/Script/Engine.PlayerController|SetbShowMouseCursor _returnvalue false)
    (Input|SetInputModeGameOnly _returnvalue false)
    (else
      ;[0.15 0.15 0.15 0.5] Is Widget Valid?
      (Utilities|IsValid (Variables|Default|GetDialogueWidget)
        (:Is%20Valid
          ;[0.15 0.15 0.15 0.5] Update Dialogue If Is Valid
          (bind _returnvalue_3 (Utilities|GetDataTableRow (Variables|Default|GetData%20Table) (Variables|Default|GetRow%20Name))
            (:then
              (Default|UpdateDialogue (Variables|Default|GetDialogueWidget) (.Dialogue (Utilities|Struct|BreakS_Dialogue _returnvalue_3)))
              (Variables|Default|SetRow%20Name (.Row (Utilities|Struct|BreakS_Dialogue _returnvalue_3)))
              (Variables|Default|SetData%20Table (.DataTable (Utilities|Struct|BreakS_Dialogue _returnvalue_3)))
              (Variables|Default|SetEndDialogue (.EndDialogue (Utilities|Struct|BreakS_Dialogue _returnvalue_3)))
              (Variables|Default|SetOpenendedDialogue (.OpenendedDialogue (Utilities|Struct|BreakS_Dialogue _returnvalue_3))))))
        (:Is%20Not%20Valid
          ;[0.15 0.15 0.15 0.5] Create Widget and Start Dialogue if Not Valid
          (bind _returnvalue_4 (Utilities|GetDataTableRow (Variables|Default|GetData%20Table) (Variables|Default|GetRow%20Name))
            (:then
              (bind _returnvalue_5 (UserInterface|CreateWidget "/Game/Dialogue/WB_Dialogue.WB_Dialogue_C" 0 (|NameToText) (.Dialogue (Utilities|Struct|BreakS_Dialogue _returnvalue_4))))
              (bind _output_get (Variables|Default|SetDialogueWidget _returnvalue_5))
              (UserInterface|Viewport|AddtoViewport _output_get 0)
              (Variables|Default|SetRow%20Name (.Row (Utilities|Struct|BreakS_Dialogue _returnvalue_4)))
              (Variables|Default|SetData%20Table (.DataTable (Utilities|Struct|BreakS_Dialogue _returnvalue_4)))
              (Variables|Default|SetEndDialogue (.EndDialogue (Utilities|Struct|BreakS_Dialogue _returnvalue_4)))
              ;[0.15 0.15 0.15 0.5] Add first widgit for options
              (Input|SetInputModeGameandUI _returnvalue_2 0 "DoNotLock" true false)
              (Variables|/Script/Engine.PlayerController|SetbShowMouseCursor _returnvalue_2 true)
              (if (.OpenendedDialogue (Utilities|Struct|BreakS_Dialogue _returnvalue_4))
                (for _array_element (.OpenendedDialogueOptions (Utilities|Struct|BreakS_Dialogue _returnvalue_4))
                  (bind _returnvalue_6 (UserInterface|CreateWidget "/Game/Dialogue/WB_Options.WB_Options_C" 0 (Utilities|Text|ToText(Name) (.OptionName (Utilities|Struct|BreakS_OptionsDialogue _array_element))) self (.Row (Utilities|Struct|BreakS_OptionsDialogue _array_element)) (.DataTable (Utilities|Struct|BreakS_OptionsDialogue _array_element))))
                  (Widget|Panel|AddChild (Variables|/Game/Dialogue/WB_Dialogue.WB_Dialogue_C|GetOptionsScrollBox (Variables|Default|GetDialogueWidget)) _returnvalue_6))))))))))

(fn ConstructionScript)