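; NPC Blueprint that runs a data-table-driven dialogue when a Character interacts with it.
; The first interaction creates a WB_Dialogue widget with the speaker name and line, and later ones update it.
; Each row supplies the next row name, table and end flag, chaining lines across tables.
; Once flagged, the next interaction removes the widget, leaving the stored row as the next conversation's start.
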(event EventInteract
  (params (Interactor :type Actor%20Object%20Reference))
  ;[0.15 0.15 0.15 0.5] Interacting with Character
  (Utilities|Casting|CastToCharacter Interactor)
  ;[0.15 0.15 0.15 0.5] Is Dialogue Ending?
  (if (Variables|Default|GetEndDialogue)
    ;[0.15 0.15 0.15 0.5] Dialogue Ended
    (Widget|RemovefromParent (Variables|Default|GetDialogueWidget))
    (Variables|Default|SetEndDialogue false)
    (Variables|Default|SetDialogueWidget 0)
    (else
      ;[0.15 0.15 0.15 0.5] Is Widget Valid?
      (Utilities|IsValid (Variables|Default|GetDialogueWidget)
        (:Is%20Valid
          ;[0.15 0.15 0.15 0.5] Update Dialogue If Is Valid
          (bind _returnvalue (Utilities|GetDataTableRow (Variables|Default|GetData%20Table) (Variables|Default|GetRow%20Name))
            (:then
              (Default|UpdateDialogue (Variables|Default|GetDialogueWidget) (.Dialogue (Utilities|Struct|BreakS_Dialogue _returnvalue)))
              (Variables|Default|SetRow%20Name (.Row (Utilities|Struct|BreakS_Dialogue _returnvalue)))
              (Variables|Default|SetData%20Table (.DataTable (Utilities|Struct|BreakS_Dialogue _returnvalue)))
              (Variables|Default|SetEndDialogue (.EndDialogue (Utilities|Struct|BreakS_Dialogue _returnvalue))))))
        (:Is%20Not%20Valid
          ;[0.15 0.15 0.15 0.5] Create Widget and Start Dialogue if Not Valid
          (bind _returnvalue_2 (Utilities|GetDataTableRow (Variables|Default|GetData%20Table) (Variables|Default|GetRow%20Name))
            (:then
              (bind _returnvalue_3 (UserInterface|CreateWidget "/Game/Dialogue/WB_Dialogue.WB_Dialogue_C" 0 (|NameToText) (.Dialogue (Utilities|Struct|BreakS_Dialogue _returnvalue_2))))
              (bind _output_get (Variables|Default|SetDialogueWidget _returnvalue_3))
              (UserInterface|Viewport|AddtoViewport _output_get 0)
              (Variables|Default|SetRow%20Name (.Row (Utilities|Struct|BreakS_Dialogue _returnvalue_2)))
              (Variables|Default|SetData%20Table (.DataTable (Utilities|Struct|BreakS_Dialogue _returnvalue_2)))
              (Variables|Default|SetEndDialogue (.EndDialogue (Utilities|Struct|BreakS_Dialogue _returnvalue_2))))))))))

(fn ConstructionScript)